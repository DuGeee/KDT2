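; BP_HelloActor is a practice actor that slides its Sphere component back and forth along relative X.
; Tick moves it by Speed times delta time, flipping IsMoveRight at 0 and 500; the flag's name is inverted, since true moves left.
; BeginPlay prints loop indices, then "fin".
; The rest is unconnected experiments with movement, rotation, printing and loops, plus an empty custom event and construction script.
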(event Custom|CustomEvent)

(event EventBeginPlay
  ;[0.1021 0.3129 0.8906] 이중 for 문
  (for _index (range 0 5)
    (Development|PrintString (Utilities|String|ToString(Integer) _index) true true "(R=0.000000,G=0.660000,B=1.000000,A=1.000000)" 6e+01))
  (Development|PrintString "fin" true true "(R=0.000000,G=0.660000,B=1.000000,A=1.000000)" 6e+01))

(event EventTick
  (params (DeltaSeconds :type Float%20%28single-precision%29))
  (bind _sphere (Variables|Default|GetSphere))
  (bind _sphere_2 (Variables|Default|GetSphere))
  (if (Variables|Default|GetIsMoveRight)
    ;[0.1434 0.7344 0.1318] 왼쪽으로 이동
    (Transformation|AddRelativeLocation _sphere (Math|Vector|MakeVector (* (* DeltaSeconds (Variables|Default|GetSpeed)) -1.0) 0.0 0.0) false false)
    (if (<= (.x (Variables|/Script/Engine.SceneComponent|GetRelativeLocation _sphere)) 0.0)
      (Variables|Default|SetIsMoveRight false))
    (else
      ;[0 0.7775 1] 오른쪽으로 이동
      (Transformation|AddRelativeLocation _sphere_2 (Math|Vector|MakeVector (* DeltaSeconds (Variables|Default|GetSpeed)) 0.0 0.0) false false)
      (if (>= (.x (Variables|/Script/Engine.SceneComponent|GetRelativeLocation _sphere_2)) 5e+02)
        (Variables|Default|SetIsMoveRight true)))))

(fn ConstructionScript)