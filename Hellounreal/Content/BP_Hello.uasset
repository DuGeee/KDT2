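; BP_Hello is an actor that slides its Sphere component back and forth along its relative X axis.
; Each Tick moves the sphere by Speed scaled by delta time, and the IsMoveLeft flag flips direction at fixed bounds of 0 and 2500.
; The per-frame rotation calls add zero, and a disconnected while loop that scales Rotation never runs.
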(event EventTick
  (params (DeltaSeconds :type Float%20%28single-precision%29))
  (bind _sphere (Variables|Default|GetSphere))
  (bind _sphere_2 (Variables|Default|GetSphere))
  (if (Variables|Default|GetIsMoveLeft)
    (Transformation|AddRelativeLocation _sphere (Math|Vector|MakeVector (* (* (Variables|Default|Getspeed) DeltaSeconds) -1.0) 0.0 0.0) false false)
    (Transformation|AddRelativeRotation _sphere (Math|Rotator|MakeRotator 0.0 0.0 0.0) false false)
    (if (<= (.x (Variables|/Script/Engine.SceneComponent|GetRelativeLocation _sphere)) 0.0)
      (Variables|Default|SetIsMoveLeft false))
    (else
      (Transformation|AddRelativeLocation _sphere_2 (Math|Vector|MakeVector (* (Variables|Default|Getspeed) DeltaSeconds) 0.0 0.0) false false)
      (Transformation|AddRelativeRotation (Variables|Default|GetSphere) (Math|Rotator|MakeRotator 0.0 0.0 0.0) false false)
      (if (>= (.x (Variables|/Script/Engine.SceneComponent|GetRelativeLocation _sphere_2)) 2.5e+03)
        (Variables|Default|SetIsMoveLeft true)))))

(fn ConstructionScript)